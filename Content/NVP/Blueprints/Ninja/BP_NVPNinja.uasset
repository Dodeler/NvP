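; Ninja character Blueprint that equips a melee weapon and plays a throw animation on input.
; On BeginPlay it spawns a BP_NinjaMeleeWeapon and snaps it to the mesh's LeftHandSocket.
; Pressing Fire only plays Throw_Montage; this graph spawns no projectile and has no hit logic.
; Overlap and Tick events are disabled stubs, and the construction script just calls its parent.
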(event EventBeginPlay
  (|CallParentFunction)
  (bind _returnvalue (Game|SpawnActorfromClass "/Game/NVP/Blueprints/Ninja/BP_NinjaMeleeWeapon.BP_NinjaMeleeWeapon_C" (Transformation|GetSocketTransform (Variables|Character|GetMesh) "LeftHandSocket" "RTS_ParentBoneSpace") "AlwaysSpawn" 0 0))
  (Transformation|AttachComponentToComponent _returnvalue (Variables|Character|GetMesh) "LeftHandSocket" "SnapToTarget" "SnapToTarget" "KeepRelative" true))

(event Collision|EventActorBeginOverlap
  (params (OtherActor :type Actor%20Object%20Reference))
  (|CallParentFunction OtherActor) ; This node is disabled and will not be called.\nDrag off pins to build functionality.
)

(event EventTick
  (params (DeltaSeconds :type Float%20%28single-precision%29))
  (|CallParentFunction DeltaSeconds) ; This node is disabled and will not be called.\nDrag off pins to build functionality.
)

(event Input|ActionEvents|InputActionFire
  (params (Key :type Key%20Structure :default "None"))
  (:Pressed
    (Animation|PlayAnimMontage "/Game/NVP/Blueprints/Ninja/Animations/Throw_Montage.Throw_Montage" 1.0 "None")))

(fn ConstructionScript
  (|CallParentFunction))